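; Pickup spawner that places a random heal, speed boost or time-low item at its own location.
; While the Spawn flag is false, Tick runs a 30-second Delay, then spawns one of the three item classes and sets the flag.
; A player character beginning overlap with the Sphere clears the flag, allowing the next timed spawn.
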(event OnComponentBeginOverlap(Sphere)
  (params (OverlappedComponent :type Primitive%20Component%20Object%20Reference) (OtherActor :type Actor%20Object%20Reference) (OtherComp :type Primitive%20Component%20Object%20Reference) (OtherBodyIndex :type Integer) (bFromSweep :type Boolean) (SweepResult :type Hit%20Result%20Structure%20%28by%20ref%29))
  (Utilities|Casting|CastToThirdPersonCharacterWithJoysticks OtherActor)
  (Variables|Default|SetSpawn? false))

(event EventTick
  (params (DeltaSeconds :type Float%20%28single-precision%29))
  (if (not (Variables|Default|GetSpawn?))
    (Utilities|FlowControl|Delay 3e+01)
    (Game|SpawnActorfromClass (Utilities|Select :Index (Math|Random|RandomInteger 3) :Option%200 "/Game/Use/BP_HPHeal.BP_HPHeal_C" :Option%201 "/Game/Use/BP_SpeedBoost.BP_SpeedBoost_C" :Option%202 "/Game/Use/BP_TimeLow.BP_TimeLow_C") (Math|Conversions|ToTransform(Vector) (Transformation|GetActorLocation)) "Undefined" 0 0)
    (Variables|Default|SetSpawn? true)))

(fn ConstructionScript)